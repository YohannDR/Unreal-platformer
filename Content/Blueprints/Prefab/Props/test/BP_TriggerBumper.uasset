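; BP_TriggerBumper is a test prop that bumps a player character upward along its owner's up vector.
; On BeginPlay, it takes the first BP_Char overlapping its Trigger and stops if none is found.
; It then calls the empty TriggerOverlapPlayer hook, passes a "None" trigger message to the character, and launches it at LaunchVelocityZ, overriding existing velocity.
; The check runs only at BeginPlay, with no overlap event or Tick logic.
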(event EventBeginPlay
  (bind _asbp_char (Utilities|Casting|CastToBP_Char (Utilities|Array|Get(acopy) (Collision|GetOverlappingActors (Variables|TriggerZone|GetTrigger) "/Game/Blueprints/Player/BP_Char.BP_Char_C" :!class /Script/Engine.Actor))))
  ;[1 1 1] Throw
  (CallFunction|TriggerOverlapPlayer 0 _asbp_char)
  (Class|AudioParameterControllerInterface|SetTriggerParameter(Message) _asbp_char "None")
  (Character|LaunchCharacter _asbp_char (* (Transformation|GetActorUpVector (Components|GetOwner)) (Variables|Default|GetLaunch%20Velocity%20Z)) true true))

(event EventTick
  (params (DeltaSeconds :type Float%20%28single-precision%29)))

(fn TriggerOverlapPlayer
  (params (Trigger :type Trigger%20Base%20Object%20Reference) (Player :type BP%20Char%20Object%20Reference)))